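; BP_PlayerBase is a player character Blueprint built around an Ability System Component and linked animation layers.
; On BeginPlay it links the ABP_Locomotion_Unarm animation class layers to its mesh for unarmed locomotion.
; Every Tick it prints two float attribute reads from the Ability System Component on screen as debug output, without logging.
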(event `self.ReceiveBeginPlay`
  (`SkeletalMeshComponent.LinkAnimClassLayers` (`self.Mesh`) "/Game/Art/AnimationAsset/PublicAnimation/ABP_Locomotion_Unarm.ABP_Locomotion_Unarm_C"))

(event `self.ReceiveTick`
  (params (DeltaSeconds :type "Float (single-precision)"))
  (`KismetSystemLibrary.PrintString` (`KismetStringLibrary.Conv_DoubleToString` (`.ReturnValue` (`AbilitySystemBlueprintLibrary.GetFloatAttributeFromAbilitySystemComponent` (`AbilitySystemBlueprintLibrary.GetAbilitySystemComponent` null) (struct :`AttributeName` "MoveSpeed" :`Attribute` "/Script/GenshinElementalWar.GenshinAttributeSet:MoveSpeed" :`AttributeOwner` "/Script/CoreUObject.Class'/Script/GenshinElementalWar.GenshinAttributeSet'")))) true false (struct :`G` 0.66 :`B` 1.0 :`A` 1.0) 0.0)
  (`KismetSystemLibrary.PrintString` (`KismetStringLibrary.Conv_DoubleToString` (`.ReturnValue` (`AbilitySystemBlueprintLibrary.GetFloatAttributeFromAbilitySystemComponent` (`AbilitySystemBlueprintLibrary.GetAbilitySystemComponent` null) (struct :`AttributeName` "Stamina" :`Attribute` "/Script/GenshinElementalWar.GenshinAttributeSet:Stamina" :`AttributeOwner` "/Script/CoreUObject.Class'/Script/GenshinElementalWar.GenshinAttributeSet'")))) true false (struct :`G` 0.66 :`B` 1.0 :`A` 1.0) 0.0))

(fn `UserConstructionScript`)